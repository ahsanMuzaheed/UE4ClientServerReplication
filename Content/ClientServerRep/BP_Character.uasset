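; Player pawn testing hand-built client-server replication of vehicle-style movement driven by throttle, steering, drag and rolling resistance.
; The owning client predicts moves and sends them to the server, then replays unacknowledged moves when the replicated state arrives.
; Simulated proxies interpolate a mesh offset between updates.
; For lag-compensated hit tests, the server rewinds the target using a capped move history and re-traces, with debug drawing and test keys.
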(event `Key|V`
  (params (Key :type "Key Structure"))
  (:`Pressed`
    (`self.K2_SetActorLocation` (+ (`self.K2_GetActorLocation`) (* (`self.GetActorForwardVector`) 1000.0)))))

(event `self.ReceiveBeginPlay`
  (set `self.guid` (`KismetGuidLibrary.NewGuid`)))

(event `Server_OnHit`
  (params (hitActor :type "/Game/ClientServerRep/BP_Character Object Reference") (moveState :type "/Game/ClientServerRep/MoveState Structure"))
  (bind _arrow (`self.Arrow`))
  (bind _returnvalue (`SceneComponent.K2_GetComponentLocation` _arrow))
  (for _array_element (`/Game/ClientServerRep/BP_Character.listServerMoveState` hitActor)
    (if (>= (`.timeStamp_8_7B30864A4F9FE8D08E13EBA6D4FBEFAD` (break `/Game/ClientServerRep/MoveState` _array_element)) moveState_timeStamp_8_7B30864A4F9FE8D08E13EBA6D4FBEFAD)
      (`|ExecutionSequence`
        (:`then_0`
          (break))
        (:`then_1`
          (`self.K2_SetActorTransform` hitActor (`.transform_11_14DE36B14C0079D35E57DD9303D39517` (break `/Game/ClientServerRep/MoveState` _array_element)) false false))
        (:`then_2`
          (`KismetSystemLibrary.DrawDebugSphere` (.location (`.transform_11_14DE36B14C0079D35E57DD9303D39517` (break `/Game/ClientServerRep/MoveState` _array_element))) 100.0 12 (struct :`R` 1.0 :`B` 0.021217 :`A` 1.0) 3.0))
        (:`then_3`
          (bind (_outhit _returnvalue_2) (`KismetSystemLibrary.LineTraceSingle` :`Start` _returnvalue :`End` (+ _returnvalue (* (`SceneComponent.GetForwardVector` _arrow) 8000.0)) :`TraceChannel` "TraceTypeQuery2" :`DrawDebugType` "ForDuration"))
          (if _returnvalue_2
            (cast `/Game/ClientServerRep/BP_Character` (`.HitActor` (`GameplayStatics.BreakHitResult` _outhit))
              (:`then`
                _)
              (:`CastFailed`
                _))
            (`KismetSystemLibrary.PrintString` (`KismetSystemLibrary.GetDisplayName` (`.HitActor` (`GameplayStatics.BreakHitResult` _outhit))))))))))

(event `InputAxis|MoveForward`
  (params (AxisValue :type "Float (single-precision)"))
  (set `self.throttle` AxisValue))

(event `Key|SpaceBar`
  (params (Key :type "Key Structure"))
  (bind _arrow (`self.Arrow`))
  (bind _returnvalue (`SceneComponent.K2_GetComponentLocation` _arrow))
  (:`Pressed`
    (bind (_outhit _returnvalue_2) (`KismetSystemLibrary.LineTraceSingle` :`Start` _returnvalue :`End` (+ _returnvalue (* (`SceneComponent.GetForwardVector` _arrow) 8000.0)) :`TraceChannel` "TraceTypeQuery2" :`DrawDebugType` "ForDuration"))
    (if _returnvalue_2
      (bind _asbp_character (cast `/Game/ClientServerRep/BP_Character` (`.HitActor` (`GameplayStatics.BreakHitResult` _outhit))))
      (`KismetSystemLibrary.PrintString` (`KismetGuidLibrary.Conv_GuidToString` (`/Game/ClientServerRep/BP_Character.guid` _asbp_character)))
      (bind _serverrepstate_lastmovestate (break `/Game/ClientServerRep/ServerRepState` (`/Game/ClientServerRep/BP_Character.serverRepState` _asbp_character)))
      (`self.Server_OnHit` _asbp_character _serverrepstate_lastmovestate))))

(event `InputAxis|MoveRight`
  (params (AxisValue :type "Float (single-precision)"))
  (set `self.steering` AxisValue))

(event `Key|R`
  (params (Key :type "Key Structure"))
  ;[1 1 1] test
  (:`Pressed`
    (set `self.autoControl` (not (`self.autoControl`)))))

(event `self.ReceiveTick`
  (params (DeltaSeconds :type "Float (single-precision)"))
  (`|ExecutionSequence`
    (:`then_0`
      ;[1 1 1] test
      (if (`self.autoControl`)
        (set `self.throttle` 1.0)
        (set `self.steering` 1.0)))
    (:`then_1`
      (`|ExecutionSequence`
        (:`then_0`
          ;[1 1 1] Set moveState and replicate to server
          (bind _output_get (set `self.moveState` (make `/Game/ClientServerRep/MoveState` DeltaSeconds (`self.steering`) (`self.throttle`) (`GameplayStatics.GetRealTimeSeconds`) (`self.GetTransform`))))
          ;;[1 1 1] (AutonomousProxy) Add moveState to list for OnRep_serverRepState validation
          (if (`self.IsLocallyControlled`)
            (`/Engine/EditorBlueprintResources/ActorMacros.Switch Has Authority`
              (:`Remote`
                (`KismetArrayLibrary.Array_Add` (`self.listClientMoveState`) _output_get)
                (`self.Server_SetMoveState` _output_get)
                (`self.SimulateMove` _output_get)))))
        (:`then_1`
          ;[1 1 1] (server) server's pawn
          (if (`|EnumEquality` (`self.GetRemoteRole`) "ROLE_SimulatedProxy")
            (`self.Server_SetMoveState` _output_get)))
        (:`then_2`
          ;[1 1 1] (SimulatedProxy) Client simulate other player's pawn
          (if (and (not (`self.IsLocallyControlled`)) (not (`self.HasAuthority`)))
            (`self.ClientUpdate` DeltaSeconds)))
        (:`then_3`
          (`KismetSystemLibrary.DrawDebugString` (`self.K2_GetActorLocation`) (`KismetGuidLibrary.Conv_GuidToString` (`self.guid`)) null (struct :`R` 1.0 :`A` 1.0)))))))

(event `Server_SetMoveState`
  (params (moveState :type "/Game/ClientServerRep/MoveState Structure"))
  (bind (_deltatime _steeering _throttle _timestamp) (break `/Game/ClientServerRep/MoveState` moveState))
  (bind _movestate (make `/Game/ClientServerRep/MoveState` _deltatime _steeering _throttle _timestamp (`self.GetTransform`)))
  ;[1 1 1] (server)
  (`self.SimulateMove` moveState)
  (`self.UpdateServerRepState` _movestate)
  (`self.AddServerMoveStateBuffer` _movestate))

(fn `AddServerMoveStateBuffer`
  (params (moveState :type "/Game/ClientServerRep/MoveState Structure (by ref)"))
  (bind _listservermovestate (`self.listServerMoveState`))
  (`KismetArrayLibrary.Array_Add` _listservermovestate moveState)
  (if (>= (`KismetArrayLibrary.Array_Length` _listservermovestate) 150)
    (`KismetArrayLibrary.Array_Remove` _listservermovestate)))

(fn `ClearListMoveState`
  (params (lastMoveState :type "/Game/ClientServerRep/MoveState Structure (by ref)"))
  (locals (tmpListMoveState :type "Array of /Game/ClientServerRep/MoveState Structure"))
  ;[1 1 1] 將server已經驗證過的moveState移除
  (for _array_element (`self.listClientMoveState`)
    (if (> (`.timeStamp_8_7B30864A4F9FE8D08E13EBA6D4FBEFAD` (break `/Game/ClientServerRep/MoveState` _array_element)) lastMoveState_timeStamp_8_7B30864A4F9FE8D08E13EBA6D4FBEFAD)
      (`KismetArrayLibrary.Array_Add` (`local.tmpListMoveState`) _array_element)))
  (set `self.listClientMoveState` (`local.tmpListMoveState`)))

(fn `ClientUpdate`
  (params (deltaTime :type "Float (double-precision)"))
  (bind (_serverrepstate_lastmovestate _serverrepstate_velocity _serverrepstate_transform) (break `/Game/ClientServerRep/ServerRepState` (`self.serverRepState`)))
  (set `self.clientTimeSinceUpdate` (+ deltaTime (`self.clientTimeSinceUpdate`)))
  ;[1 1 1] Don't update, if update too fast
  (if (>= (`self.clientTimeBetweenUpdate`) (`self.KINDA_SMALL_NUMBER`))
    ;[1 1 1] Interpolate current transform to target
    (`SceneComponent.K2_SetWorldTransform` (`self.MeshOffset`) (`KismetMathLibrary.TLerp` (`self.clientStartTransform`) _serverrepstate_transform (/ (`self.clientTimeSinceUpdate`) (`self.clientTimeBetweenUpdate`)) "DualQuatInterp") false false)))

(fn `OnRep_serverRepState`
  (bind (_serverrepstate_lastmovestate _serverrepstate_velocity _serverrepstate_transform) (break `/Game/ClientServerRep/ServerRepState` (`self.serverRepState`)))
  (bind (_serverrepstate_lastmovestate_2 _serverrepstate_velocity_2 _serverrepstate_transform_2) (break `/Game/ClientServerRep/ServerRepState` (`self.serverRepState`)))
  (if (`self.HasAuthority`)
    _
    (elif (`self.IsLocallyControlled`)
      ;[1 1 1] AutonomousProxy
      (set `self.velocity` _serverrepstate_velocity)
      (`self.K2_SetActorTransform` _serverrepstate_transform)
      (`self.ClearListMoveState` _serverrepstate_lastmovestate)
      (for _array_element (`self.listClientMoveState`)
        (`self.SimulateMove` _array_element))
      (else
        ;[1 1 1] SimulatedProxy
        (set `self.clientTimeBetweenUpdate` (`self.clientTimeSinceUpdate`))
        (set `self.clientTimeSinceUpdate` 0.0)
        (set `self.clientStartTransform` (`SceneComponent.K2_GetComponentToWorld` (`self.MeshOffset`)))
        (`self.K2_SetActorTransform` _serverrepstate_transform_2)
        (set `self.velocity` _serverrepstate_velocity_2)))))

(fn `SimulateMove`
  (params (moveState :type "/Game/ClientServerRep/MoveState Structure (by ref)"))
  (`self.UpdateRotation` moveState_deltaTime_2_CDC2054D444B450CA5D0069CC8F12DF4 moveState_steeering_4_6302E799445203C77FD0399CB82BE2A3)
  (`self.UpdateLocation` moveState_deltaTime_2_CDC2054D444B450CA5D0069CC8F12DF4 moveState_throttle_6_10DBD7204BC13BBC1512DD852BB7AA0B))

(fn `UpdateLocation`
  (params (deltaTime :type "Float (double-precision)") (throttle :type "Float (double-precision)"))
  ;[1 1 1] Update location from velocity
  (bind _output_get (set `self.velocity` (+ (`self.velocity`) (* (/ (+ (* (`self.GetActorForwardVector`) (* throttle (`self.maxForce`))) (* (`KismetMathLibrary.Normal` (`self.velocity`)) (* (`KismetMathLibrary.VSizeSquared` (`self.velocity`)) (`self.dragCoefficient`))) (* (`KismetMathLibrary.Normal` (`self.velocity`)) (* (`self.mass`) (`self.rollingCoefficient`) 9.8))) (`self.mass`)) deltaTime))))
  (bind _sweephitresult (`self.K2_AddActorWorldOffset` (* _output_get (* deltaTime 100.0)) true))
  (if (`GameplayStatics.BreakHitResult` _sweephitresult)
    (set `self.velocity` (0.0 0.0 0.0))))

(fn `UpdateRotation`
  (params (deltaTime :type "Float (double-precision)") (steering :type "Float (double-precision)"))
  (bind _returnvalue (`KismetMathLibrary.MakeRotator` 0.0 0.0 (* steering (/ (* deltaTime (`KismetMathLibrary.Dot_VectorVector` (`self.GetActorForwardVector`) (`self.velocity`))) (`self.turingRadius`)))))
  (`self.K2_AddActorWorldRotation` _returnvalue)
  (set `self.velocity` (`KismetMathLibrary.GreaterGreater_VectorRotator` (`self.velocity`) _returnvalue)))

(fn `UpdateServerRepState`
  (params (lastMoveState :type "/Game/ClientServerRep/MoveState Structure (by ref)"))
  (set `self.serverRepState` (make `/Game/ClientServerRep/ServerRepState` lastMoveState (`self.velocity`) (`self.GetTransform`))))

(fn `UserConstructionScript`)